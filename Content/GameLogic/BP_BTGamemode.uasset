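; BP_BTGamemode is a game mode that tracks a score and shows it on screen through the BPW_Score widget.
; On BeginPlay it creates the score widget for the first player and adds it to the viewport.
; The A_PointWon event adds a fixed amount to ATotalPoints and copies the total into the widget.
; A G key press runs the same scoring logic.
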(event `self.ReceiveBeginPlay`
  ;[1 1 1] Create Widgwt Score
  (bind _returnvalue (`|CreateWidget` "/Game/UI/BPW_Score.BPW_Score_C" (`GameplayStatics.GetPlayerController` 0)))
  (bind _output_get (set `self.ScoreWidgetRef` _returnvalue))
  (`UserWidget.AddToViewport` _output_get 0))

(event `Key|G`
  (params (Key :type "Key Structure"))
  (:`Pressed`
    (bind _output_get (set `self.A_TotalPoints` (+ (`self.A_TotalPoints`) 15) :!label _label))
    (set `/Game/UI/BPW_Score.A_ScorePoints` _output_get (`self.ScoreWidgetRef`))))

(event `A_PointWon`
  (goto _label))

(fn `UserConstructionScript`)