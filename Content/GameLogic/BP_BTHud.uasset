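; HUD Blueprint that keeps a tennis-style match score for sides A and B and creates the score and main-menu widgets.
; Debug-style keys award points through MultiGates stepping 15/30/40/game, feeding games, up to three recorded sets, server swaps and a 6-6 tiebreak.
; A function-name timer counts match seconds, stopping at 10.
; G and L quick-save and load match variables through a SaveInfoBT slot, though some set fields are miswired.
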(event `CloseSet`
  ;[0.4565 0.8898 1] Set Logic
  (set `self.Set_Index` (+ (`self.Set_Index`) 1) :!label _label)
  (`self.ResetPoints`)
  (switch `int` (`self.Set_Index`)
    (:`1`
      (set `self.Current_A_Set` (`self.Current_A_Games`))
      (set `self.Current_B_Set` (`self.Current_B_Games`)))
    (:`2`
      (set `self.Current_A_Set_2` (`self.Current_A_Games`))
      (set `self.Current_B_Set_2` (`self.Current_B_Games`)))
    (:`3`
      (set `self.Current_A_Set_3` (`self.Current_A_Games`))
      (set `self.Current_B_Set_3` (`self.Current_B_Games`))))
  (`self.ResetPoints`)
  (`|ExecutionSequence`
    (:`then_0`
      (set `self.Current_A_Points` 0))
    (:`then_1`
      (set `self.Current_B_Points` 0))
    (:`then_2`
      (set `self.Current_A_Games` 0))
    (:`then_3`
      (set `self.Current_B_Games` 0))))

(event `self.ReceiveBeginPlay`
  (`self.StartGameNow`)
  (`|ExecutionSequence`
    (:`then_0`
      ;[1 0.8917 0.161] Create Widgwt Score
      (bind _returnvalue (`|CreateWidget` "/Game/UI/BPW_Score.BPW_Score_C" (`GameplayStatics.GetPlayerController` 0)))
      (bind _output_get (set `self.BPW_ScoreReference` _returnvalue))
      (`UserWidget.AddToViewport` _output_get 0)
      (`self.BTStartGame`))
    (:`then_1`
      ;[0.3512 0.7811 1] Create Button Pause Menu in viewport
      (bind _returnvalue_2 (`|CreateWidget` "/Game/UI/BPW_Menu_MainScreen.BPW_Menu_MainScreen_C"))
      (bind _output_get_2 (set `self.BPW_MainMunuReference` _returnvalue_2))
      (`UserWidget.AddToViewport` _output_get_2 0)
      (`Widget.SetVisibility` _output_get_2 "Visible")
      (`WidgetBlueprintLibrary.SetInputMode_GameAndUIEx` (`GameplayStatics.GetPlayerController` 0) _output_get_2 "DoNotLock" false))))

(event `Key|N`
  (params (Key :type "Key Structure"))
  (bind _current_a_games (`self.Current_A_Games`))
  (bind _current_b_games (`self.Current_B_Games`))
  (bind _current_a_games_2 (`self.Current_A_Games`))
  (bind _current_b_games_2 (`self.Current_B_Games`))
  ;[0.1382 0.3466 1] CountPoints
  (:`Pressed`
    (`self.GetPoints`)
    (if (`self.CurrentTieBreak?`)
      (`self.Tie_Point_A`)
      (else
        (`|MultiGate` false true :!label _label_2
          (:`Out 0`
            (set `self.Current_A_Points` (+ (`self.Current_A_Points`) 15)))
          (:`Out 1`
            (set `self.Current_A_Points` (+ (`self.Current_A_Points`) 15)))
          (:`Out 2`
            (set `self.Current_A_Points` (+ (`self.Current_A_Points`) 10)))
          (:`Out 3`
            (set `self.Current_A_Games` (+ (`self.Current_A_Games`) 1))
            (set `self.Current_A_Points` 0)
            (set `self.Current_B_Points` 0)
            (`|ExecutionSequence` :!label _label_3
              (:`then_0`
                ;[0.4565 0.8898 1] Set Logic
                (if (or (and (== _current_a_games_2 6) (<= _current_b_games_2 4)) (and (== _current_b_games_2 6) (<= _current_a_games_2 4)))
                  (`|ExecutionSequence`
                    (:`then_0`
                      (goto _label)))
                  (elif (or (and (== _current_a_games 7) (<= _current_b_games 5)) (and (== _current_b_games 7) (<= _current_a_games 5)))
                    (`self.CloseSet`))))
              (:`then_1`
                ;[1 0.3291 0.2794] Server SET
                (set `self.Current_A_Server` (not (`self.Current_A_Server`)))
                (set `self.Current_B_Server` (not (`self.Current_B_Server`)))
                (`self.ResetPoints`)))))))))

(event `GetPoints`
  ;[1 0.9471 0.3642] TieBreak ?
  (if (and (== (`self.Current_A_Games`) 6) (== (`self.Current_B_Games`) 6))
    (set `self.CurrentTieBreak?` true)))

(event `ResetPoints`
  ;[0.1382 0.3466 1] CountPoints
  (`|ExecutionSequence`
    (:`then_0`
      (goto _label_2 :!via `Reset`))
    (:`then_1`
      (goto _label_5 :!via `Reset`))))

(event `Key|V`
  (params (Key :type "Key Structure"))
  ;[0.04688 0.002546 0.02238] Para teste de mudanca dos dados
  (:`Pressed`
    (set `self.Current_A_Set` (+ (`self.Current_A_Set`) 1))
    (set `self.Current_B_Set` (+ (`self.Current_B_Set`) 1))
    (set `self.Current_A_Games` (+ (`self.Current_A_Games`) 1))
    (set `self.Current_B_Games` (+ (`self.Current_B_Games`) 1))
    (set `self.Current_A_Points` (+ (`self.Current_A_Points`) 1))
    (set `self.Current_B_Points` (+ (`self.Current_B_Points`) 1))
    (set `self.CurrentTotalTime` (+ (`self.CurrentTotalTime`) 1))
    (set `self.Current_A_Server` (not (`self.Current_A_Server`)))
    (set `self.Current_B_Server` (not (`self.Current_B_Server`)))))

(event `Tie_Point_A`
  (bind _current_a_points (`self.Current_A_Points`))
  (bind _current_b_points (`self.Current_B_Points`))
  ;[0.5547 0.4792 1] TieBreak Logic
  (bind _result (`/Engine/EditorBlueprintResources/StandardMacros.IncrementInt` (`self.Current_A_Points`))
    (:`  `
      (bind _output_get (set `self.Current_A_Points` _result))
      (if (== (mod (+ _output_get (stale `Tie_Point_B` _output_get)) 2) 1) :!label _label_4
        (`|ExecutionSequence`
          (:`then_0`
            (if (and (or (>= _current_a_points 7) (>= _current_b_points 7)) (!= (- _current_a_points _current_b_points) 1))
              (if (> (`self.Current_A_Points`) (`self.Current_B_Points`))
                (set `self.Current_A_Games` 7)
                (set `self.Current_B_Games` 6)
                (else
                  (set `self.Current_A_Games` 6)
                  (set `self.Current_B_Games` 7)))
              (`self.CloseSet`)
              (`self.ResetPoints`)
              (set `self.CurrentTieBreak?` false)))
          (:`then_1`
            ;;[1 0.3291 0.2794] Server SET
            (set `self.Current_A_Server` (not (`self.Current_A_Server`)))
            (set `self.Current_B_Server` (not (`self.Current_B_Server`)))))))))

(event `Tie_Point_B`
  ;[0.5547 0.4792 1] TieBreak Logic
  (bind _result (`/Engine/EditorBlueprintResources/StandardMacros.IncrementInt` (`self.Current_B_Points`))
    (:`  `
      (bind _output_get (set `self.Current_B_Points` _result))
      (goto _label_4))))

(event `Key|M`
  (params (Key :type "Key Structure"))
  ;[0.1382 0.3466 1] CountPoints
  (:`Pressed`
    (`self.GetPoints`)
    (if (`self.CurrentTieBreak?`)
      (`self.Tie_Point_B`)
      (else
        (`|MultiGate` false true :!label _label_5
          (:`Out 0`
            (set `self.Current_B_Points` (+ (`self.Current_B_Points`) 15)))
          (:`Out 1`
            (set `self.Current_B_Points` (+ (`self.Current_B_Points`) 15)))
          (:`Out 2`
            (set `self.Current_B_Points` (+ (`self.Current_B_Points`) 10)))
          (:`Out 3`
            (set `self.Current_B_Games` (+ (`self.Current_B_Games`) 1))
            (set `self.Current_B_Points` 0)
            (set `self.Current_A_Points` 0)
            (goto _label_3)))))))

(event `Key|Enter`
  (params (Key :type "Key Structure"))
  ;[1 0.1689 0.142] Start GAME - Para funcionar input no HUD BP
  (:`Pressed`
    (`self.BTStartGame`)
    (`GameplayStatics.PlaySoundAtLocation` null (0.001 0.0 0.0) (struct) 1.0 1.0 0.0 null null null :!label _label_6)))

(event `StartGameNow`
  ;[1 0.1689 0.142] Start GAME - Para funcionar input no HUD BP
  (`self.BTStartGame`)
  (`self.EnableInput` (`GameplayStatics.GetPlayerController` 0))
  (goto _label_6))

(event `Clock`
  (bind _currenttotaltime (`self.CurrentTotalTime`))
  ;[1 1 1] Timer Clock
  (set `self.CurrentTotalTime` (+ _currenttotaltime 1))
  (if (== _currenttotaltime 10)
    (`KismetSystemLibrary.K2_ClearTimer` null "Clock")))

(event `Key|G`
  (params (Key :type "Key Structure"))
  ;[0.3615 1 0.6415] BT Quick Save
  (:`Pressed`
    (bind _returnvalue (`GameplayStatics.DoesSaveGameExist` "SlotBT"))
    (if _returnvalue
      (bind _returnvalue_2 (`GameplayStatics.LoadGameFromSlot` "SlotBT"))
      (bind _assave_info_bt (cast `/Game/Misc/SaveInfoBT` _returnvalue_2))
      (set `self.SaveInfoBTVar` _assave_info_bt)
      (`self.SaveGameVars`)
      (`GameplayStatics.SaveGameToSlot` (`self.SaveInfoBTVar`) "SlotBT")
      (`KismetSystemLibrary.PrintString` "SALVO EM Existente")
      (else
        (bind _returnvalue_3 (`GameplayStatics.CreateSaveGameObject` "/Game/Misc/SaveInfoBT.SaveInfoBT_C"))
        (set `self.SaveInfoBTVar` _returnvalue_3)
        (`self.SaveGameVars`)
        (`GameplayStatics.SaveGameToSlot` (`self.SaveInfoBTVar`) "SlotBT")
        (`KismetSystemLibrary.PrintString` "JOGO SALVO")))))

(event `Key|L`
  (params (Key :type "Key Structure"))
  ;[1 1 1] Quick Load
  (:`Pressed`
    (bind _returnvalue (`GameplayStatics.DoesSaveGameExist` "SlotBT"))
    (if _returnvalue
      (bind _returnvalue_2 (`GameplayStatics.LoadGameFromSlot` "SlotBT"))
      (bind _assave_info_bt (cast `/Game/Misc/SaveInfoBT` _returnvalue_2))
      (set `self.SaveInfoBTVar` _assave_info_bt)
      (`self.LoadGameVars`)
      (`KismetSystemLibrary.PrintString` "JogoLIDO")
      (else
        (`KismetSystemLibrary.PrintString` "SEMJOGOSALVO")))))

(fn `UserConstructionScript`)